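; BP_Player is the player pawn Blueprint, handling movement through Enhanced Input.
; On BeginPlay it adds the IMC_PlayerInput mapping context to the first player controller's subsystem.
; Horizontal and vertical move actions add movement input along the HorizontalDirection and VerticalDirection variables.
; Both then share one rotation step that sets yaw only, derived from those directions scaled by input, snapping the actor toward its movement.
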(event Input|EnhancedActionEvents|EnhancedInputActionIA_MoveHorizontal
  (params (ActionValue :type Vector%202D%20Structure) (ElapsedSeconds :type Float%20%28double-precision%29) (TriggeredSeconds :type Float%20%28double-precision%29) (InputAction :type Input%20Action%20Object%20Reference :default "/Game/A_StudyContent/BluePrint/Input/IA_MoveHorizontal.IA_MoveHorizontal"))
  (bind _x (Math|Vector2D|BreakVector2D ActionValue))
  (bind _horizontaldirection (Variables|Default|GetHorizontalDirection))
  ;[0.15 0.15 0.15 0.5] 移动
  (Pawn|Input|AddMovementInput _horizontaldirection _x false)
  (Transformation|SetActorRotation (Math|Rotator|MakeRotator 0.0 0.0 (.Yaw (Math|Rotator|BreakRotator (Math|Rotator|MakeRotfromX (+ (* _horizontaldirection _x) (* (Variables|Default|GetVerticalDirection) (.X (Math|Vector2D|BreakVector2D (stale Input|EnhancedActionEvents|EnhancedInputActionIA_MoveVertical ActionValue)))))))))))

(event Input|EnhancedActionEvents|EnhancedInputActionIA_MoveVertical
  (params (ActionValue :type Vector%202D%20Structure) (ElapsedSeconds :type Float%20%28double-precision%29) (TriggeredSeconds :type Float%20%28double-precision%29) (InputAction :type Input%20Action%20Object%20Reference :default "/Game/A_StudyContent/BluePrint/Input/IA_MoveVertical.IA_MoveVertical"))
  (bind _x (Math|Vector2D|BreakVector2D ActionValue))
  (bind _verticaldirection (Variables|Default|GetVerticalDirection))
  ;[0.15 0.15 0.15 0.5] 移动
  (Pawn|Input|AddMovementInput _verticaldirection _x false)
  (Transformation|SetActorRotation (Math|Rotator|MakeRotator 0.0 0.0 (.Yaw (Math|Rotator|BreakRotator (Math|Rotator|MakeRotfromX (+ (* (Variables|Default|GetHorizontalDirection) (.X (Math|Vector2D|BreakVector2D (stale Input|EnhancedActionEvents|EnhancedInputActionIA_MoveHorizontal ActionValue)))) (* _verticaldirection _x))))))))

(event EventBeginPlay
  (Input|AddMappingContext (PlayerController|LocalPlayerSubsystems|GetEnhancedInputLocalPlayerSubsystem (Game|GetPlayerController 0)) "/Game/A_StudyContent/BluePrint/Input/IMC_PlayerInput.IMC_PlayerInput" 0 "(bIgnoreAllPressedKeysUntilRelease=True,bForceImmediately=False,bNotifyUserSettings=False)"))

(event Collision|EventActorBeginOverlap
  (params (OtherActor :type Actor%20Object%20Reference)))

(event EventTick
  (params (DeltaSeconds :type Float%20%28single-precision%29)))

(fn ConstructionScript)